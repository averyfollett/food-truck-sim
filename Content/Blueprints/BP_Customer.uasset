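; BP_Customer is a customer that creates its own cone order and a tray linked to that order.
; On BeginPlay it spawns BP_Order as a child actor, sets itself as the order's customer and adds a cone to it.
; It then spawns an offset BP_Tray child actor and passes it the order.
; ProcessOrder checks whether the tray is complete and only prints a debug message; nothing here calls it.
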(event EventBeginPlay
  (bind _order (CallFunction|AddOrder))
  (CallFunction|AddTray _order))

(fn ConstructionScript)

(fn AddOrder
  (bind _returnvalue (AddComponent|AddChildActorComponent false))
  (bind _asbp_order (Utilities|Casting|CastToBP_Order (Variables|/Script/Engine.ChildActorComponent|GetChildActor _returnvalue)))
  (Variables|Default|SetOrder _asbp_order)
  (Variables|/Game/Blueprints/BP_Order.BP_Order_C|Setcustomer _asbp_order self)
  (Development|PrintString "order added" true true "(R=0.000000,G=0.660000,B=1.000000,A=1.000000)" 1e+01)
  (Default|AddCone _asbp_order)
  (return _asbp_order))

(fn AddTray
  (params (Order :type BP%20Order%20Object%20Reference))
  (bind _returnvalue (AddComponent|AddChildActorComponent false (Math|Transform|MakeTransform "-150.000000, 0, 0")))
  (bind _asbp_tray (Utilities|Casting|CastToBP_Tray (Variables|/Script/Engine.ChildActorComponent|GetChildActor _returnvalue)))
  (Variables|Default|SetTray _asbp_tray)
  (Variables|/Game/Blueprints/BP_Tray.BP_Tray_C|Setorder _asbp_tray Order))

(fn ProcessOrder
  (if (Variables|/Game/Blueprints/BP_Tray.BP_Tray_C|GetisComplete (Variables|Default|GetTray))
    (Development|PrintString "YAY THE ORDER IS DONE" true true "(R=0.000000,G=0.660000,B=1.000000,A=1.000000)" 1e+01)))