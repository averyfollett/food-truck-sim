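; BP_Tray is a carryable tray that collects food items and checks their cone flavors against an order.
; Hit components tagged Interactible on actors of accepted classes get attached to the tray and stored in ItemArray.
; Every Tick, CheckOrderIsComplete compares each ordered cone with each stored one, only printing per-pair results; older checks sit unconnected.
; BP_MotionController's Pickup disables physics and attaches the tray; Drop reverses this.
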(event OnComponentHit(Tray)
  (params (HitComponent :type Primitive%20Component%20Object%20Reference) (OtherActor :type Actor%20Object%20Reference) (OtherComp :type Primitive%20Component%20Object%20Reference) (NormalImpulse :type Vector :default "0, 0, 0") (Hit :type Hit%20Result%20Structure%20%28by%20ref%29))
  ;[1 1 1] attach item to tray if it is a food/drink item
  (for _array_element (Variables|Default|GetacceptableItemClasses)
    (if (and (Components|ComponentHasTag OtherComp "Interactible") (== (Utilities|GetClass OtherActor) _array_element))
      (Transformation|AttachComponentToComponent OtherActor (Variables|Default|GetTray) "None" "KeepWorld" "KeepWorld" "KeepRelative" true)
      (bind _asbp_item (Utilities|Casting|CastToBP_Item OtherActor))
      (Utilities|Array|Add (Variables|Default|GetitemArray) _asbp_item)
      (Development|PrintString (Utilities|String|Append (Utilities|GetDisplayName _asbp_item) "added to tray") true true "(R=0.000000,G=0.660000,B=1.000000,A=1.000000)" 1e+01))))

(event EventTick
  (params (DeltaSeconds :type Float%20%28single-precision%29))
  (CallFunction|CheckOrderIsComplete))

(event EventPickup
  (params (AttachTo :type Scene%20Component%20Object%20Reference))
  ;[1 1 1] pickup and drop
  (Physics|SetSimulatePhysics (Variables|Default|GetTray) false)
  (Transformation|AttachComponentToComponent (VehicleSound|GetRootComponent) AttachTo "None" "KeepWorld" "KeepWorld" "KeepWorld" false))

(event EventDrop
  ;[1 1 1] pickup and drop
  (Physics|SetSimulatePhysics (Variables|Default|GetTray) true)
  (Transformation|DetachFromActor "KeepWorld" "KeepWorld" "KeepWorld"))

(fn ConstructionScript)

(fn CheckOrderIsComplete
  (for _array_element (Variables|/Game/Blueprints/BP_Order.BP_Order_C|GetconeStructArray (Variables|Default|Getorder))
    (for _array_element_2 (Variables|Default|GetitemArray)
      (bind _asbp_cone (Utilities|Casting|CastToBP_Cone _array_element_2))
      (if (Utilities|Enum|Equal(Enum) (Variables|/Game/Blueprints/BP_Cone.BP_Cone_C|Getflavor _asbp_cone) (.Flavor (Utilities|Struct|BreakST_Cone _array_element)))
        (Development|PrintString "Item found" true true "(R=0.038735,G=1.000000,B=0.000000,A=1.000000)" 1e+01)
        (else
          (Development|PrintString "Order NOT Correct" true true "(R=1.000000,G=0.000000,B=0.000000,A=1.000000)" 1e+01))))))