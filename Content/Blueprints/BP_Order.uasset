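; BP_Order is a VR order slip actor that can be picked up by motion controllers and holds an array of order items.
; Pickup disables physics on the OrderSlip and attaches the root to the controller's component, while Drop restores physics and detaches.
; AddCone creates a child actor component, casts its actor to BP_Cone, calls GenerateCone and appends it to ItemArray, with debug prints.
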(event EventPickup
  (params (AttachTo :type Scene%20Component%20Object%20Reference))
  ;[1 1 1] pickup and drop
  (Physics|SetSimulatePhysics (Variables|Default|GetOrderSlip) false)
  (Transformation|AttachComponentToComponent (VehicleSound|GetRootComponent) AttachTo "None" "KeepWorld" "KeepWorld" "KeepWorld" false))

(event EventDrop
  ;[1 1 1] pickup and drop
  (Physics|SetSimulatePhysics (Variables|Default|GetOrderSlip) true)
  (Transformation|DetachFromActor "KeepWorld" "KeepWorld" "KeepWorld"))

(fn ConstructionScript)

(fn AddCone
  (bind _returnvalue (AddComponent|AddChildActorComponent false))
  (bind _asbp_cone (Utilities|Casting|CastToBP_Cone (Variables|/Script/Engine.ChildActorComponent|GetChildActor _returnvalue)))
  (Development|PrintString "cone added" true true "(R=0.000000,G=0.660000,B=1.000000,A=1.000000)" 1e+01)
  (Default|GenerateCone _asbp_cone)
  (Development|PrintString "cone generated" true true "(R=0.000000,G=0.660000,B=1.000000,A=1.000000)" 1e+01)
  (Utilities|Array|Add (Variables|Default|GetitemArray) _asbp_cone))