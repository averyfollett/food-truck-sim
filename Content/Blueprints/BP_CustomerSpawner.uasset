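; BP_CustomerSpawner is an actor that spawns a BP_Customer at its own location when play begins.
; BeginPlay copies NumCustomersToSpawn into a remaining counter and, if that is positive, spawns one customer with collision adjustment, decrements the counter and prints a debug message.
; The check runs once with no loop or timer, so only one customer spawns regardless of the configured count.
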(event EventBeginPlay
  (Variables|Default|SetnumCustomersRemaining (Variables|Default|GetnumCustomersToSpawn))
  (if (> (Variables|Default|GetnumCustomersRemaining) 0)
    (Game|SpawnActorfromClass "/Game/Blueprints/BP_Customer.BP_Customer_C" (Math|Conversions|ToTransform(Vector) (Transformation|GetActorLocation)) "AdjustIfPossibleButAlwaysSpawn" 0 0)
    (Math|Integer|DecrementInt (Variables|Default|GetnumCustomersRemaining)
      (:%20%20
        (Development|PrintString "customer spawned" true true "(R=0.000000,G=0.660000,B=1.000000,A=1.000000)" 1e+01)))))

(fn ConstructionScript)