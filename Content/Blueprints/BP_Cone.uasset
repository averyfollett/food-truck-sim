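; BP_Cone is an ice cream cone Blueprint that generates a random flavor and addon combination.
; Its GenerateCone event calls AddRandomFlavor and AddRandomAddon, each appending one random enum value to FlavorArray or AddonArray.
; Random picks span the enum's entry count, and each result is printed for debugging.
; Nothing in this graph calls GenerateCone, and BeginPlay only runs the parent.
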(event Custom|GenerateCone
  (Development|PrintString "Generating Cone")
  (CallFunction|AddRandomFlavor)
  (CallFunction|AddRandomAddon))

(event EventBeginPlay
  (|CallParentFunction))

(event Collision|EventActorBeginOverlap
  (params (OtherActor :type Actor%20Object%20Reference))
  (|CallParentFunction OtherActor) ; This node is disabled and will not be called.\nDrag off pins to build functionality.
)

(event EventTick
  (params (DeltaSeconds :type Float%20%28single-precision%29))
  (|CallParentFunction DeltaSeconds) ; This node is disabled and will not be called.\nDrag off pins to build functionality.
)

(fn ConstructionScript
  (|CallParentFunction))

(fn AddRandomFlavor
  (bind _flavorarray (Variables|Default|GetflavorArray))
  (bind _returnvalue (Utilities|Array|Add _flavorarray (Utilities|Enum|ByteToEnumEN_IceCreamFlavors (Math|Conversions|ToByte(Integer) (Math|Random|RandomIntegerinRange 0 (- (|GetNumEnumEntries) 1))))))
  (Development|PrintString (Utilities|String|EnumtoString (Utilities|Array|Get(acopy) _flavorarray _returnvalue))))

(fn AddRandomAddon
  (bind _addonarray (Variables|Default|GetaddonArray))
  (bind _returnvalue (Utilities|Array|Add _addonarray (Utilities|Enum|ByteToEnumEN_IceCreamAddons (Math|Conversions|ToByte(Integer) (Math|Random|RandomIntegerinRange 0 (- (|GetNumEnumEntries) 1))))))
  (Development|PrintString (Utilities|String|EnumtoString (Utilities|Array|Get(acopy) _addonarray _returnvalue))))